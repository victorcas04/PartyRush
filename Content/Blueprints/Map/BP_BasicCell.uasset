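; BP_BasicCell is a map cell Blueprint with a base visual and a selection highlight visual, each tinted and scaled through setter events.
; BeginPlay creates dynamic materials for both visuals, caches the cell size and applies the selected color.
; Selection runs two timelines that ping-pong by reversing on finish, pulsing the highlight's opacity and scale.
; Deselection stops both timelines, zeroes highlight opacity and sets the base visual to its original size.
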(event `self.ReceiveBeginPlay`
  (`|ExecutionSequence`
    (:`then_0`
      (bind _returnvalue (`PrimitiveComponent.CreateDynamicMaterialInstance` (`self.CellVisual2D`) 0 null "None"))
      (set `self.BP_BaseMI` _returnvalue))
    (:`then_1`
      (bind _returnvalue_2 (`PrimitiveComponent.CreateDynamicMaterialInstance` (`self.CellSelectedVisual2D`) 0 null "None"))
      (set `self.BP_SelectedMI` _returnvalue_2))
    (:`then_2`
      (set `self.OriginalSize` (`self.Cell_GetSize`))
      (`self.SetSelectedColor` (`self.SelectedColor`)))))

(event `self.BP_SetCellColor`
  (params (NewColor :type "LinearColor Structure"))
  (bind _bp_basemi (`self.BP_BaseMI`)
    (:`then`
      (`MaterialInstanceDynamic.SetVectorParameterValue` _bp_basemi "Color" NewColor))
    (:`else`)))

(event `SetSelectedColor`
  (params (NewColor :type "LinearColor Structure"))
  (bind _bp_selectedmi (`self.BP_SelectedMI`)
    (:`then`
      (`MaterialInstanceDynamic.SetVectorParameterValue` _bp_selectedmi "Color" NewColor))
    (:`else`)))

(event `self.BP_SetCellSize`
  (params (NewSize :type "Float (single-precision)"))
  (bind _returnvalue (/ NewSize 100.0))
  (`SceneComponent.SetRelativeScale3D` (`self.CellVisual2D`) (`KismetMathLibrary.MakeVector` _returnvalue _returnvalue 1.0)))

(event `SetSelectedSize`
  (params (NewSize :type "Float (double-precision)"))
  (bind _returnvalue (/ NewSize 100.0))
  (`SceneComponent.SetRelativeScale3D` (`self.CellSelectedVisual2D`) (`KismetMathLibrary.MakeVector` _returnvalue _returnvalue 1.0)))

(event `self.BP_SetCellSelected`
  (params (bSelected :type Boolean))
  (`|ExecutionSequence`
    (:`then_0`
      (if bSelected
        (bind (_direction _selectedeffectcurve_color) (`Timeline|SelectedEffect_Color` :!via `ReverseFromEnd` :!label _label)
          (:`Update`
            (`MaterialInstanceDynamic.SetScalarParameterValue` (`self.BP_SelectedMI`) "Opacity" _selectedeffectcurve_color))
          (:`Finished`
            (switch `ETimelineDirection` _direction
              (:`Forward`
                (goto _label :!via `ReverseFromEnd`))
              (:`Backward`
                (goto _label :!via `PlayFromStart`)))))
        (else
          (`|ExecutionSequence`
            (:`then_0`
              (goto _label :!via `Stop`))
            (:`then_1`
              (`MaterialInstanceDynamic.SetScalarParameterValue` (`self.BP_SelectedMI`) "Opacity" 0.0))))))
    (:`then_1`
      (if bSelected
        (bind (_direction_2 _selectedeffectcurve_size) (`Timeline|SelectedEffect_Size` :!via `ReverseFromEnd` :!label _label_2)
          (:`Update`
            (`self.SetSelectedSize` (* (+ 1.0 (* _selectedeffectcurve_size (`self.SizeMux`))) (`self.OriginalSize`))))
          (:`Finished`
            (switch `ETimelineDirection` _direction_2
              (:`Forward`
                (goto _label_2 :!via `ReverseFromEnd`))
              (:`Backward`
                (goto _label_2 :!via `PlayFromStart`)))))
        (else
          (`|ExecutionSequence`
            (:`then_0`
              (goto _label_2 :!via `Stop`))
            (:`then_1`
              (`self.BP_SetCellSize` (`KismetMathLibrary.Conv_IntToDouble` (`self.OriginalSize`))))))))))

(fn `UserConstructionScript`)