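; Player controller that translates input actions for selection, menu and four-way directional navigation into same-named calls.
; A parallel set of Menu-prefixed actions keeps menu selection and navigation separate from the regular controls.
; Select and menu actions fire on release, while directional actions fire on press.
; The graph only forwards input, with no state checks or other logic, and the construction script is empty.
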(event `InputAction|Select`
  (params (Key :type "Key Structure"))
  (:`Released`
    (`self.Select`)))

(event `InputAction|Menu`
  (params (Key :type "Key Structure"))
  (:`Released`
    (`self.Menu`)))

(event `InputAction|Menu_Select`
  (params (Key :type "Key Structure"))
  (:`Released`
    (`self.Menu_Select`)))

(event `InputAction|Up`
  (params (Key :type "Key Structure"))
  (:`Pressed`
    (`self.Up`)))

(event `InputAction|Down`
  (params (Key :type "Key Structure"))
  (:`Pressed`
    (`self.Down`)))

(event `InputAction|Right`
  (params (Key :type "Key Structure"))
  (:`Pressed`
    (`self.Right`)))

(event `InputAction|Left`
  (params (Key :type "Key Structure"))
  (:`Pressed`
    (`self.Left`)))

(event `InputAction|Menu_Up`
  (params (Key :type "Key Structure"))
  (:`Pressed`
    (`self.Menu_Up`)))

(event `InputAction|Menu_Down`
  (params (Key :type "Key Structure"))
  (:`Pressed`
    (`self.Menu_Down`)))

(event `InputAction|Menu_Right`
  (params (Key :type "Key Structure"))
  (:`Pressed`
    (`self.Menu_Right`)))

(event `InputAction|Menu_Left`
  (params (Key :type "Key Structure"))
  (:`Pressed`
    (`self.Menu_Left`)))

(fn `UserConstructionScript`)