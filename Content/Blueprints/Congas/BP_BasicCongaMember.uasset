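; Visual actor for a single conga member, using a base mesh and a selection mesh, each with a dynamic material for color, scaled relative to cell size.
; Selection loops ping-pong timelines: the lead pulses the overlay's color and size, other members pulse the base mesh's size.
; Merging fades the overlay from merge color to member color, staggered by member index.
; Move feedback is a stub that only applies the staggered delay.
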(event `self.ReceiveBeginPlay`
  (`|ExecutionSequence`
    (:`then_0`
      (bind _returnvalue (`PrimitiveComponent.CreateDynamicMaterialInstance` (`self.CongaMemberVisual3D`) 0 null "None"))
      (set `self.BP_BaseMI` _returnvalue))
    (:`then_1`
      (bind _returnvalue_2 (`PrimitiveComponent.CreateDynamicMaterialInstance` (`self.CongaMemberSelectedVisual3D`) 0 null "None"))
      (set `self.BP_SelectedMI` _returnvalue_2))
    (:`then_2`
      (set `self.OriginalSize` (`self.CongaMember_GetSize`))
      (`SceneComponent.SetVisibility` (`self.CongaMemberSelectedVisual3D`) false false))))

(event `self.BP_SetCongaMemberColor`
  (params (NewColor :type "LinearColor Structure"))
  (bind _bp_basemi (`self.BP_BaseMI`)
    (:`then`
      (`MaterialInstanceDynamic.SetVectorParameterValue` _bp_basemi "Color" NewColor))
    (:`else`)))

(event `self.BP_AdjustZPos`
  (bind (_returnvalue_x _returnvalue_y) (`KismetMathLibrary.BreakVector` (`self.K2_GetActorLocation`)))
  (`self.K2_SetActorLocation` (`KismetMathLibrary.MakeVector` _returnvalue_x _returnvalue_y (* (/ (* (`self.CongaMember_GetSize`) (`self.MemberToCellRelation`)) 100.0) (`self.GetOriginalZPos`)))))

(event `SetSelectedColor`
  (params (NewColor :type "LinearColor Structure"))
  (bind _bp_selectedmi (`self.BP_SelectedMI`)
    (:`then`
      (`MaterialInstanceDynamic.SetVectorParameterValue` _bp_selectedmi "Color" NewColor))
    (:`else`)))

(event `self.BP_SetCongaMemberSize`
  (params (NewSize :type "Float (single-precision)"))
  (`SceneComponent.SetRelativeScale3D` (`self.CongaMemberVisual3D`) (`KismetMathLibrary.Conv_DoubleToVector` (/ (* NewSize (`self.MemberToCellRelation`)) 100.0))))

(event `SetSelectedSize`
  (params (NewSize :type "Float (double-precision)"))
  (`SceneComponent.SetRelativeScale3D` (`self.CongaMemberSelectedVisual3D`) (`KismetMathLibrary.Conv_DoubleToVector` (/ (* NewSize (`self.MemberToCellRelation`)) 100.0))))

(event `self.BP_SetCongaMemberSelected`
  (params (bSelected :type Boolean) (bLead :type Boolean))
  (`|ExecutionSequence`
    (:`then_0`
      (if bLead
        (if bSelected
          (`SceneComponent.SetVisibility` (`self.CongaMemberSelectedVisual3D`) true false)
          (bind (_direction _selectedeffectcurve_color) (`Timeline|Timeline_0` :!via `ReverseFromEnd` :!label _label)
            (:`Update`
              (`self.SetSelectedColor` (`KismetMathLibrary.LinearColorLerp` (`self.GetColor`) (`self.SelectedColor`) _selectedeffectcurve_color)))
            (:`Finished`
              (switch `ETimelineDirection` _direction
                (:`Forward`
                  (goto _label :!via `ReverseFromEnd`))
                (:`Backward`
                  (goto _label :!via `PlayFromStart`)))))
          (else
            (`|ExecutionSequence`
              (:`then_0`
                (goto _label :!via `Stop`))
              (:`then_1`
                (`SceneComponent.SetVisibility` (`self.CongaMemberSelectedVisual3D`) false false)
                (`self.SetSelectedColor` (`self.SelectedColor`))))))))
    (:`then_1`
      (if bSelected
        (bind (_direction_2 _selectedeffectcurve_size) (`Timeline|Timeline_1` :!via `ReverseFromEnd` :!label _label_2)
          (:`Update`
            (if bLead
              (bind _returnvalue (* (+ 1.0 (* _selectedeffectcurve_size (`self.SizeMux`))) (`self.OriginalSize`)))
              (`self.SetSelectedSize` _returnvalue)
              (else
                (`self.BP_SetCongaMemberSize` _returnvalue))))
          (:`Finished`
            (switch `ETimelineDirection` _direction_2
              (:`Forward`
                (goto _label_2 :!via `ReverseFromEnd`))
              (:`Backward`
                (goto _label_2 :!via `PlayFromStart`)))))
        (else
          (`|ExecutionSequence`
            (:`then_0`
              (goto _label_2 :!via `Stop`))
            (:`then_1`
              (`self.BP_SetCongaMemberSize` (`KismetMathLibrary.Conv_IntToDouble` (`self.OriginalSize`))))))))))

(event `self.BP_CongaMemberMoved`
  (params (MemberIdx :type Integer))
  (bind _returnvalue (* (`self.TimeBeforeMoveFeedback`) MemberIdx))
  (if (> _returnvalue 0.0)
    (`KismetSystemLibrary.Delay` _returnvalue)))

(event `self.BP_CongaMemberMerged`
  (params (MemberIdx :type Integer))
  (bind _returnvalue (* (`self.TimeBeforeMergeFeedback`) MemberIdx))
  (`SceneComponent.SetVisibility` (`self.CongaMemberSelectedVisual3D`) true false)
  (if (> _returnvalue 0.0)
    (`KismetSystemLibrary.Delay` _returnvalue)
    (bind (_direction _mergedeffectcurve_color) (`Timeline|Timeline_2` :!via `PlayFromStart` :!label _label_3)
      (:`Update`
        (`self.SetSelectedColor` (`KismetMathLibrary.LinearColorLerp` (`self.MergeColor`) (`self.GetColor`) _mergedeffectcurve_color)))
      (:`Finished`
        (`SceneComponent.SetVisibility` (`self.CongaMemberSelectedVisual3D`) false false)
        (`self.BP_SetCongaMemberColor` (`self.GetColor`))))
    (else
      (goto _label_3 :!via `PlayFromStart`))))

(fn `UserConstructionScript`)